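; BP_enemy is a spinning obstacle enemy that damages the player on contact and awards score when shot.
; Tick yaws the Enemy component at RotationSpeed, while a separate PassDetect volume destroys the actor once the player passes through it.
; Capsule overlaps reduce player health and update the HUD, or on lethal hits reset score and show the restart screen.
; Projectile overlaps add score via the player controller; every such hit destroys the enemy.
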(event `self.ReceiveTick`
  (params (DeltaSeconds :type "Float (single-precision)"))
  (`SceneComponent.K2_AddLocalRotation` (`self.Enemy`) (`KismetMathLibrary.MakeRotator` 0.0 0.0 (* DeltaSeconds (`self.RotationSpeed`))) false false))

(event `self.PassDetect.OnComponentBeginOverlap`
  (params (OverlappedComponent :type "PrimitiveComponent Object Reference") (OtherActor :type "Actor Object Reference") (OtherComp :type "PrimitiveComponent Object Reference") (OtherBodyIndex :type Integer) (bFromSweep :type Boolean) (SweepResult :type "HitResult Structure (by ref)"))
  (cast `/Game/InfiniteMatrix/Blueprints/BP_Player` OtherActor)
  (`self.K2_DestroyActor`))

(event `self.Capsule.OnComponentBeginOverlap`
  (params (OverlappedComponent :type "PrimitiveComponent Object Reference") (OtherActor :type "Actor Object Reference") (OtherComp :type "PrimitiveComponent Object Reference") (OtherBodyIndex :type Integer) (bFromSweep :type Boolean) (SweepResult :type "HitResult Structure (by ref)"))
  (`|ExecutionSequence`
    (:`then_0`
      (bind _asbp_player (cast `/Game/InfiniteMatrix/Blueprints/BP_Player` OtherActor)
        (:`then`
          (bind _returnvalue (- (`/Game/InfiniteMatrix/Blueprints/BP_Player.CurrentHealth` _asbp_player) 10.0))
          (if (> _returnvalue 0.0)
            (bind _output_get (set `/Game/InfiniteMatrix/Blueprints/BP_Player.CurrentHealth` _returnvalue _asbp_player))
            (bind _playercontroller (`/Game/InfiniteMatrix/Blueprints/BP_Player.PlayerController` _asbp_player))
            (`/Game/InfiniteMatrix/Blueprints/BP_player_controller.SetHealth` _playercontroller _output_get (`/Game/InfiniteMatrix/Blueprints/BP_Player.MaxHealth` _asbp_player))
            (`self.K2_DestroyActor`)
            (else
              (set `/Game/InfiniteMatrix/Blueprints/BP_Player.Score` 0 _asbp_player)
              (`/Game/InfiniteMatrix/Blueprints/BP_player_controller.RemoveHealthBarFromViewport` _playercontroller)
              (`/Game/InfiniteMatrix/Blueprints/BP_Player.DisplayRestart` _asbp_player)
              (`self.K2_DestroyActor`))))
        (:`CastFailed`
          (cast `/Game/InfiniteMatrix/Blueprints/BP_Projectile` OtherActor)
          (bind _asbp_player_2 (cast `/Game/InfiniteMatrix/Blueprints/BP_Player` (`GameplayStatics.GetPlayerPawn` 0)))
          (bind _output_get_2 (set `/Game/InfiniteMatrix/Blueprints/BP_Player.Score` (+ (`/Game/InfiniteMatrix/Blueprints/BP_Player.Score` _asbp_player_2) 10) _asbp_player_2))
          (`/Game/InfiniteMatrix/Blueprints/BP_player_controller.SetScore` (`/Game/InfiniteMatrix/Blueprints/BP_Player.PlayerController` _asbp_player_2) _output_get_2)
          (`self.K2_DestroyActor` self))))))

(fn `UserConstructionScript`)