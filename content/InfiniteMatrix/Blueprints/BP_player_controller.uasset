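; Player controller Blueprint that owns the main HUD widget for health and score display.
; On BeginPlay it creates WB_main if none exists, stores the reference and adds it to the viewport.
; SetHealth and SetScore forward values to that widget, and RemoveHealthBarFromViewport takes it off screen.
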(event `self.ReceiveBeginPlay`
  (`self.ShowHealthBar`))

(fn `RemoveHealthBarFromViewport`
  (`Widget.RemoveFromParent` (`self.WBMain`)))

(fn `SetHealth`
  (params (CurrentHealth :type "Float (double-precision)") (MaxHealth :type "Float (double-precision)"))
  (`/Game/InfiniteMatrix/UI/WB_main.SetHealthBar` (`self.WBMain`) CurrentHealth MaxHealth))

(fn `SetScore`
  (params (Score :type Integer))
  (`/Game/InfiniteMatrix/UI/WB_main.SetScore` (`self.WBMain`) Score))

(fn `ShowHealthBar`
  (`/Engine/EditorBlueprintResources/StandardMacros.IsValid` (`self.WBMain`)
    (:`Is Valid`
      _)
    (:`Is Not Valid`
      (bind _returnvalue (`|CreateWidget` "/Game/InfiniteMatrix/UI/WB_main.WB_main_C"))
      (bind _output_get (set `self.WBMain` _returnvalue))))
  (`UserWidget.AddToViewport` _output_get 0))

(fn `UserConstructionScript`)