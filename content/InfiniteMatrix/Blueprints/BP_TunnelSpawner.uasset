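; Spawner actor that builds the tunnel out of chained BP_Tunnel segments and populates it with pickups and enemies.
; On BeginPlay it destroys existing tunnels and their health packs, then spawns a short run starting at the player pawn when no valid newest tunnel exists.
; Each new segment attaches at the previous one's SpawnPoint, stores a spawner reference and randomizes its walls.
; Segments get randomly placed enemies and sometimes a randomly rotated health pack.
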(event `self.ReceiveBeginPlay`
  (`self.SpawnInitialTunnels`))

(fn `SpawnInitialTunnels`
  (`|ExecutionSequence`
    (:`then_0`
      (bind _outactors (`GameplayStatics.GetAllActorsOfClass` "/Game/InfiniteMatrix/Blueprints/BP_Tunnel.BP_Tunnel_C"))
      (for _array_element _outactors
        (bind _healthpackreference (`/Game/InfiniteMatrix/Blueprints/BP_Tunnel.HealthPackReference` _array_element))
        (`/Engine/EditorBlueprintResources/StandardMacros.IsValid` _healthpackreference
          (:`Is Valid`
            (`self.K2_DestroyActor` _healthpackreference))
          (:`Is Not Valid`
            _))
        (`self.K2_DestroyActor` _array_element)))
    (:`then_1`
      (for _ (range 3)
        (`/Engine/EditorBlueprintResources/StandardMacros.IsValid` (`self.NewestTunnel`)
          (:`Is Valid`
            (`self.SpawnTunnelAtSpawnPoint`))
          (:`Is Not Valid`
            (`self.SpawnTunnel` (`self.K2_GetActorLocation` (`GameplayStatics.GetPlayerPawn` 0)))))))))

(fn `SpawnTunnel`
  (params (SpawnLocation :type "Vector Structure"))
  (bind _returnvalue (`KismetMathLibrary.RandomFloatInRange` 0.0 360.0))
  (bind _returnvalue_2 (`|SpawnActorFromClass` "/Game/InfiniteMatrix/Blueprints/BP_Tunnel.BP_Tunnel_C" (`KismetMathLibrary.MakeTransform` SpawnLocation) "Undefined" "MultiplyWithRoot" null null))
  (bind _output_get (set `self.NewestTunnel` _returnvalue_2))
  (set `/Game/InfiniteMatrix/Blueprints/BP_Tunnel.TunnelSpawner` self _output_get)
  (`/Game/InfiniteMatrix/Blueprints/BP_Tunnel.RandomizeWall` _output_get)
  (if (== (`KismetMathLibrary.RandomIntegerInRange` 8 9) 9)
    (bind _returnvalue_3 (`|SpawnActorFromClass` "/Game/InfiniteMatrix/Blueprints/BP_Health_Pack.BP_Health_Pack_C" (`KismetMathLibrary.MakeTransform` (+ SpawnLocation (`KismetMathLibrary.MakeVector` (`KismetMathLibrary.RandomFloatInRange` 100.0 2200.0) (`KismetMathLibrary.RandomFloatInRange` -300.0 300.0) (`KismetMathLibrary.RandomFloatInRange` -300.0 300.0))) (struct :`Pitch` 60.0 :`Roll` 30.0)) "Undefined" "MultiplyWithRoot" null null))
    (set `/Game/InfiniteMatrix/Blueprints/BP_Tunnel.HealthPackReference` _returnvalue_3 (`self.NewestTunnel`))
    (`SceneComponent.K2_AddLocalRotation` (`/Game/InfiniteMatrix/Blueprints/BP_Health_Pack.HealthPack` _returnvalue_3) (`KismetMathLibrary.MakeRotator` _returnvalue _returnvalue) false false))
  (if (== (`KismetMathLibrary.RandomIntegerInRange` 4 4) 4)
    (for _ (range (+ (`KismetMathLibrary.RandomIntegerInRange` 0 2) 1))
      (bind _returnvalue_4 (`|SpawnActorFromClass` "/Game/InfiniteMatrix/Blueprints/BP_enemy.BP_enemy_C" (`KismetMathLibrary.MakeTransform` (+ SpawnLocation (`KismetMathLibrary.MakeVector` (`KismetMathLibrary.RandomFloatInRange` 100.0 2200.0) (`KismetMathLibrary.RandomFloatInRange` -300.0 300.0) (`KismetMathLibrary.RandomFloatInRange` -300.0 300.0)))) "Undefined" "MultiplyWithRoot" null null))
      (set `/Game/InfiniteMatrix/Blueprints/BP_enemy.PlayerReferenceFromEnemy` null _returnvalue_4))))

(fn `SpawnTunnelAtSpawnPoint`
  (`self.SpawnTunnel` (`SceneComponent.K2_GetComponentLocation` (`/Game/InfiniteMatrix/Blueprints/BP_Tunnel.SpawnPoint` (`self.NewestTunnel`)))))

(fn `UserConstructionScript`)