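; BP_Tunnel is an endless tunnel segment with a rotating wall that BP_Player must pass through.
; RandomizeWall picks one of four hole meshes and tints it pink or red when player health is low.
; Touching the wall calls ProcessHit on the player and turns it red.
; The trigger zone asks TunnelSpawner for another segment, destroys this one and any referenced health pack, and awards a point if the wall was untouched.
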(event `self.ReceiveTick`
  (params (DeltaSeconds :type "Float (single-precision)"))
  (`SceneComponent.K2_AddLocalRotation` (`self.WallMesh`) (`KismetMathLibrary.MakeRotator` (* DeltaSeconds (`self.RotateSpeed`))) false false))

(event `self.TriggerZone.OnComponentBeginOverlap`
  (params (OverlappedComponent :type "PrimitiveComponent Object Reference") (OtherActor :type "Actor Object Reference") (OtherComp :type "PrimitiveComponent Object Reference") (OtherBodyIndex :type Integer) (bFromSweep :type Boolean) (SweepResult :type "HitResult Structure (by ref)"))
  (bind _healthpackreference (`self.HealthPackReference`))
  (bind _asbp_player (cast `/Game/InfiniteMatrix/Blueprints/BP_Player` OtherActor))
  (`/Game/InfiniteMatrix/Blueprints/BP_TunnelSpawner.SpawnTunnelAtSpawnPoint` (`self.TunnelSpawner`))
  (`/Engine/EditorBlueprintResources/StandardMacros.IsValid` _healthpackreference
    (:`Is Valid`
      (`self.K2_DestroyActor` _healthpackreference))
    (:`Is Not Valid`
      _))
  (`self.K2_DestroyActor`)
  (if (not (`self.CollideWithWall`))
    (bind _output_get (set `/Game/InfiniteMatrix/Blueprints/BP_Player.Score` (+ 1 (`/Game/InfiniteMatrix/Blueprints/BP_Player.Score` _asbp_player)) _asbp_player))
    (`/Game/InfiniteMatrix/Blueprints/BP_player_controller.SetScore` (`/Game/InfiniteMatrix/Blueprints/BP_Player.PlayerController` _asbp_player) _output_get)))

(event `self.WallMesh.OnComponentBeginOverlap`
  (params (OverlappedComponent :type "PrimitiveComponent Object Reference") (OtherActor :type "Actor Object Reference") (OtherComp :type "PrimitiveComponent Object Reference") (OtherBodyIndex :type Integer) (bFromSweep :type Boolean) (SweepResult :type "HitResult Structure (by ref)"))
  (bind _asbp_player (cast `/Game/InfiniteMatrix/Blueprints/BP_Player` OtherActor))
  (`/Game/InfiniteMatrix/Blueprints/BP_Player.ProcessHit` _asbp_player)
  (set `self.CollideWithWall` true)
  (`PrimitiveComponent.SetMaterial` (`self.WallMesh`) 0 "/Game/InfiniteMatrix/Materials/MI_Red.MI_Red"))

(fn `RandomizeWall`
  (bind _wallmesh (`self.WallMesh`))
  (`StaticMeshComponent.SetStaticMesh` (`self.WallMesh`) (select `int` (`KismetMathLibrary.RandomIntegerInRange` 0 3) :`0` "/Game/InfiniteMatrix/Meshes/SM_Hole_01.SM_Hole_01" :`1` "/Game/InfiniteMatrix/Meshes/SM_Hole_02.SM_Hole_02" :`2` "/Game/InfiniteMatrix/Meshes/SM_Hole_03.SM_Hole_03" :`3` "/Game/InfiniteMatrix/Meshes/SM_Hole_04.SM_Hole_04" :!type "StaticMesh Object Reference"))
  (`SceneComponent.K2_AddLocalRotation` (`self.WallMesh`) (`KismetMathLibrary.MakeRotator` 0.0) false false)
  (bind _asbp_player (cast `/Game/InfiniteMatrix/Blueprints/BP_Player` (`GameplayStatics.GetPlayerPawn` 0)))
  (bind _currenthealth (`/Game/InfiniteMatrix/Blueprints/BP_Player.CurrentHealth` _asbp_player))
  (if (< _currenthealth 10.0)
    (`PrimitiveComponent.SetMaterial` _wallmesh 0 "/Game/InfiniteMatrix/Materials/MI_Red.MI_Red")
    (elif (< _currenthealth 20.0)
      (`PrimitiveComponent.SetMaterial` _wallmesh 0 "/Game/InfiniteMatrix/Materials/MI_Pink.MI_Pink"))))

(fn `UserConstructionScript`)